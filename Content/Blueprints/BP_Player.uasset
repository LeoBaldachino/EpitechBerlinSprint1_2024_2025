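; Player character with Enhanced Input move and look, a hold-to-charge jump and wall riding.
; Tick traces to the character's right, deriving wall normal and ride direction.
; Jumping while falling beside a wall starts the ride, which switches to Flying and launches along the wall each frame.
; Jump hold time scales launch force on release, with a Niagara charge effect and an ABP_Beats animation flag.
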(event `self.ReceiveTick`
  (params (DeltaSeconds :type "Float (single-precision)"))
  (bind _outhit (`KismetSystemLibrary.LineTraceSingle` (`self.K2_GetActorLocation`) (+ (* (`self.GetActorRightVector`) (`self.WallDetectionDistance`)) (`self.K2_GetActorLocation`)) "TraceTypeQuery1"))
  (bind _output_get (set `self.WallNormal ` (`.Normal` (`GameplayStatics.BreakHitResult` _outhit))))
  (bind _output_get_2 (set `self.WallRideDirection` (`KismetMathLibrary.Cross_VectorVector` (`KismetMathLibrary.MakeVector` 0.0 0.0 1.0) _output_get)))
  (`self.WallRiding` 0.0))

(event `WallRiding`
  (params (DeltaSeconds :type "Float (single-precision)"))
  ;[1 1 1] Wall Riding
  ;;[1 1 1] Force player to stick to wall while wall ride is active
  (if (`self.IsWallRiding`)
    (set `self.WallRideStartPoint` (`self.K2_GetActorLocation`))
    (`self.AddMovementInput` (`self.WallRideDirection`) (`self.WallRideSpeed `))
    (`self.K2_SetActorLocation` (`KismetMathLibrary.VInterpTo` (`self.K2_GetActorLocation`) (- (`self.K2_GetActorLocation`) (* (`self.WallNormal `) (`KismetMathLibrary.Dot_VectorVector` (- (`self.K2_GetActorLocation`) (`self.WallRideStartPoint`)) (`self.WallNormal `)))) (`GameplayStatics.GetWorldDeltaSeconds`) 10.0) true)
    ;;[1 1 1] Disable Movement & Force player to stick to the wall
    (`CharacterMovementComponent.DisableMovement` (`self.CharacterMovement`))
    (`CharacterMovementComponent.SetMovementMode` (`self.CharacterMovement`) "MOVE_Flying" 0)
    (`self.LaunchCharacter` (* (`self.WallRideDirection`) (`self.WallRideSpeed `)) true true)
    (`self.K2_SetActorRotation` (`KismetMathLibrary.Conv_VectorToRotator` (`self.WallRideDirection`)))))

(event `EnhancedInput|/Game/Input/Action/IA_MyJump`
  (params (ActionValue :type Boolean) (ElapsedSeconds :type "Float (double-precision)") (TriggeredSeconds :type "Float (double-precision)") (InputAction :type "InputAction Object Reference" :default "/Game/Input/Action/IA_MyJump.IA_MyJump"))
  (:`Triggered`
    (if (`KismetMathLibrary.NotEqualExactly_VectorVector` (`self.WallNormal `))
      (if (`NavMovementComponent.IsFalling` (`self.CharacterMovement`))
        (set `self.IsWallRiding` true)))))

(event `self.ReceiveBeginPlay`
  (bind _returnvalue (pcsubsystem `EnhancedInputLocalPlayerSubsystem` (`self.GetLocalViewingPlayerController`)))
  ;[1 1 1] Controller init
  (`/Engine/EditorBlueprintResources/StandardMacros.IsValid` _returnvalue
    (:`Is Valid`
      (`EnhancedInputSubsystemInterface.AddMappingContext` _returnvalue "/Game/Input/IMC_PLAYER.IMC_PLAYER" 0 (struct)))))

(event `EnhancedInput|/Game/Input/Action/IA_MyJump`
  (params (ActionValue :type Boolean) (ElapsedSeconds :type "Float (double-precision)") (TriggeredSeconds :type "Float (double-precision)") (InputAction :type "InputAction Object Reference" :default "/Game/Input/Action/IA_MyJump.IA_MyJump"))
  (bind _returnvalue (`SkeletalMeshComponent.GetAnimInstance` (`self.Mesh`)))
  ;[1 1 1] Jump Animation
  (:`Triggered`
    (if (`NavMovementComponent.IsFalling` (`self.CharacterMovement`))
      _
      (elif (`self.IsWallRiding`)
        (set `self.IsWallRiding` false)
        (elif true
          (bind _asabp_beats (cast `/Game/Characters/ABP_Beats` _returnvalue))
          (set `/Game/Characters/ABP_Beats.isHoldingSpace` true _asabp_beats)))))
  (:`Completed`
    (bind _asabp_beats_2 (cast `/Game/Characters/ABP_Beats` _returnvalue))
    (set `/Game/Characters/ABP_Beats.isHoldingSpace` false _asabp_beats_2)))

(event `EnhancedInput|/Game/Input/Action/IA_MyJump`
  (params (ActionValue :type Boolean) (ElapsedSeconds :type "Float (double-precision)") (TriggeredSeconds :type "Float (double-precision)") (InputAction :type "InputAction Object Reference" :default "/Game/Input/Action/IA_MyJump.IA_MyJump"))
  ;[1 1 1] Jump with holding space
  (:`Started`
    (if (`NavMovementComponent.IsMovingOnGround` (`self.CharacterMovement`))
      (set `self.IsJumping` true)
      (set `self.JumpStartTime` (`KismetSystemLibrary.GetGameTimeInSeconds`))
      (`NiagaraFunctionLibrary.SpawnSystemAttached` "/Game/Particles/ChargingJump.ChargingJump" (`self.NSC_LeftFoot`) "None" (0.0 0.0 0.0) (struct) "KeepRelativeOffset")))
  (:`Completed`
    (set `self.IsJumping` false)
    (if (not (`NavMovementComponent.IsFalling` (`self.CharacterMovement`)))
      (`self.LaunchCharacter` (`KismetMathLibrary.MakeVector` 0.0 0.0 (`KismetMathLibrary.Lerp` (`self.MinJumpForce`) (`self.MaxJumpForce`) (/ (`KismetMathLibrary.FClamp` (- (`KismetSystemLibrary.GetGameTimeInSeconds`) (`self.JumpStartTime`)) 0.0 (`self.MaxHoldTime`)) (`self.MaxHoldTime`)))) false true)
      (`ActorComponent.Deactivate` (`self.NSC_LeftFoot`))
      (`ActorComponent.Deactivate` (`self.NSC_RightFoot`)))))

(event `EnhancedInput|/Game/Input/Action/IA_MyLook`
  (params (ActionValue :type "Vector2D Structure") (ElapsedSeconds :type "Float (double-precision)") (TriggeredSeconds :type "Float (double-precision)") (InputAction :type "InputAction Object Reference" :default "/Game/Input/Action/IA_MyLook.IA_MyLook"))
  ;[1 1 1] Camera tilt
  (:`Triggered`
    (`self.AddControllerPitchInput` ActionValue_Y)
    (`self.AddControllerYawInput` ActionValue_X)))

(event `EnhancedInput|/Game/Input/Action/IA_MyMove`
  (params (ActionValue :type "Vector2D Structure") (ElapsedSeconds :type "Float (double-precision)") (TriggeredSeconds :type "Float (double-precision)") (InputAction :type "InputAction Object Reference" :default "/Game/Input/Action/IA_MyMove.IA_MyMove"))
  (bind (_returnvalue_roll _returnvalue_pitch _returnvalue_yaw) (`KismetMathLibrary.BreakRotator` (`self.GetControlRotation`)))
  (bind (_returnvalue_roll_2 _returnvalue_pitch_2 _returnvalue_yaw_2) (`KismetMathLibrary.BreakRotator` (`self.GetControlRotation`)))
  ;[1 1 1] Movement
  (:`Triggered`
    (`self.AddMovementInput` (`KismetMathLibrary.GetRightVector` (`KismetMathLibrary.MakeRotator` 0.0 0.0 _returnvalue_yaw_2)) ActionValue_X)
    (`self.AddMovementInput` (`KismetMathLibrary.GetForwardVector` (`KismetMathLibrary.MakeRotator` 0.0 0.0 _returnvalue_yaw)) ActionValue_Y)))

(fn `UserConstructionScript`)