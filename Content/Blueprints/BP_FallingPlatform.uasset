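; BP_FallingPlatform is a platform that drops when the player steps on it and then resets.
; An overlap on its Box by player character 0 starts a timed chain of delays that swaps the Cube's material to warning looks before enabling physics so it falls.
; After a short fall it disables physics, teleports back to the transform saved at BeginPlay and restores its default material.
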(event `self.ReceiveBeginPlay`
  (set `self.OG POS` (`SceneComponent.K2_GetComponentToWorld` (`self.Cube`))))

(event `self.Box.OnComponentBeginOverlap`
  (params (OverlappedComponent :type "PrimitiveComponent Object Reference") (OtherActor :type "Actor Object Reference") (OtherComp :type "PrimitiveComponent Object Reference") (OtherBodyIndex :type Integer) (bFromSweep :type Boolean) (SweepResult :type "HitResult Structure (by ref)"))
  (if (== OtherActor (`GameplayStatics.GetPlayerCharacter` 0))
    (`PrimitiveComponent.SetMaterial` (`self.Cube`) 0 "/Engine/MapTemplates/Materials/BasicAsset01.BasicAsset01")
    (`KismetSystemLibrary.Delay` 1.5)
    (`PrimitiveComponent.SetMaterial` (`self.Cube`) 0 "/Game/Materials/FallingAlert_Inst.FallingAlert_Inst")
    (`KismetSystemLibrary.Delay` 0.5)
    (`PrimitiveComponent.SetSimulatePhysics` (`self.Cube`) true)
    (`KismetSystemLibrary.Delay` 1.0)
    (`PrimitiveComponent.SetSimulatePhysics` (`self.Cube`) false)
    (`SceneComponent.K2_SetWorldTransform` (`self.Cube`) (`self.OG POS`) false true)
    (`PrimitiveComponent.SetMaterial` (`self.Cube`) 0 "/Engine/BasicShapes/BasicShapeMaterial.BasicShapeMaterial")))

(fn `UserConstructionScript`)