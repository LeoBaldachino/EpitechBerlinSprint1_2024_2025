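; BP_CP is a Sonic-style checkpoint prop that sets the player's respawn point when touched.
; On BP_Player overlap while inactive, it stores and prints its location as CurrentRespawnPoint, calls SetAllDisabledEvent on itself, then marks itself activated.
; Activation swaps one mesh material to green and plays a 2D sound.
; SetAllDisabled_Event restores the default material and clears the activated flag.
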(event `self.ReceiveActorBeginOverlap`
  (params (OtherActor :type "Actor Object Reference"))
  (bind _asbp_player (cast `/Game/Blueprints/BP_Player` OtherActor))
  (if (not (`self.activated`))
    (bind _output_get (set `/Game/Blueprints/BP_Player.CurrentRespawnPoint` (`self.K2_GetActorLocation`) _asbp_player))
    (`KismetSystemLibrary.PrintString` (`KismetStringLibrary.Conv_VectorToString` _output_get))
    (`self.SetAllDisabled_Event` (cast `/Game/Levels/Props/Obstacles/BP_CP` self :!pure true))
    (set `self.activated` true)
    (`PrimitiveComponent.SetMaterial` (`self.Sonic_Checkpoint`) 5 "/Engine/EngineDebugMaterials/VertexColorViewMode_GreenOnly.VertexColorViewMode_GreenOnly")
    (`GameplayStatics.PlaySound2D` "/Game/Levels/Props/Obstacles/sonic-checkpoint.sonic-checkpoint" 1.0 1.0 0.0 null null)))

(event `SetAllDisabled_Event`
  (`PrimitiveComponent.SetMaterial` (`self.Sonic_Checkpoint`) 5 "/Game/Levels/Props/Build/lambert6.lambert6")
  (set `self.activated` false))

(fn `UserConstructionScript`)